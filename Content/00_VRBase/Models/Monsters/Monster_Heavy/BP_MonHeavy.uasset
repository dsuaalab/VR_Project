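; Heavy monster for a VR game that takes damage and can deal fixed damage to an assigned door.
; BeginPlay scales HP by a Weight multiplier, which GetRound sets by round number, then spawns a separate health bar actor.
; Damage plays a sound and updates the bar's fill.
; Tick keeps the bar above the monster facing the player camera, and destroys both actors when HP runs out.
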(event `self.ReceiveBeginPlay`
  (`|ExecutionSequence`
    (:`then_0`
      (set `self.Init_HP` (* (`self.weight`) (`self.Init_HP`)))
      (set `self.HP` (* (`self.weight`) (`self.HP`))))
    (:`then_1`
      (bind _returnvalue (`|SpawnActorFromClass` "/Game/00_VRBase/Models/Monsters/MonsterHPBar_BP.MonsterHPBar_BP_C" (`KismetMathLibrary.MakeTransform` (`SceneComponent.K2_GetComponentLocation` (`self.Cube_HpBarPoseDummy`))) "Undefined" "OverrideRootScale" null null))
      (set `self.MonsterHpBarActor` _returnvalue)
      (bind _asmonster_hpbar (cast `/Game/00_VRBase/Models/Monsters/MonsterHPBar` (`WidgetComponent.GetUserWidgetObject` (`/Game/00_VRBase/Models/Monsters/MonsterHPBar_BP.HPBarComp` (`self.MonsterHpBarActor`)))))
      (bind _output_get (set `self.Monster HPBar UI` _asmonster_hpbar))
      (`/Game/00_VRBase/Models/Monsters/MonsterHPBar.setHpPercent` _output_get (/ (`self.HP`) (`self.Init_HP`))))))

(event `self.ReceiveTick`
  (params (DeltaSeconds :type "Float (single-precision)"))
  (bind _monsterhpbaractor (`self.MonsterHpBarActor`))
  (if (<= (`self.HP`) 0.0)
    (`self.K2_DestroyActor` _monsterhpbaractor)
    (`self.K2_DestroyActor`)
    (else
      (`/Game/00_VRBase/Models/Monsters/MonsterHPBar_BP.UpdateLocation` _monsterhpbaractor (`SceneComponent.K2_GetComponentLocation` (`self.Cube_HpBarPoseDummy`)))
      (`/Game/00_VRBase/Models/Monsters/MonsterHPBar_BP.UpdateRotation` _monsterhpbaractor (`KismetMathLibrary.FindLookAtRotation` (`self.K2_GetActorLocation` (`self.MonsterHpBarActor`)) (`self.K2_GetActorLocation` (`GameplayStatics.GetPlayerCameraManager` 0)))))))

(event `GetRound`
  (params (round :type Integer))
  (switch `int` round
    (:`1`
      (set `self.weight` 3.0))
    (:`2`
      (set `self.weight` 1.5))))

(event `self.ReceiveAnyDamage`
  (params (Damage :type "Float (single-precision)") (DamageType :type "DamageType Object Reference") (InstigatedBy :type "Controller Object Reference") (DamageCauser :type "Actor Object Reference"))
  (`AudioComponent.Play` (`self.Audio`) 0.0)
  (set `self.HP` (- (`self.HP`) Damage))
  (set `/Game/00_VRBase/Models/Monsters/MonsterHPBar.HpPercent` (/ (`self.HP`) (`self.Init_HP`)) (`self.Monster HPBar UI`)))

(event `SetDoorData`
  (params (door :type "/Game/00_VRBase/Models/Castle_Door/BP_Castle_Door Object Reference"))
  (set `self.door` door))

(event `GiveDamage`
  (`GameplayStatics.ApplyDamage` (`self.door`) 50.0))

(fn `OnRep_mon_door`)

(fn `UserConstructionScript`)