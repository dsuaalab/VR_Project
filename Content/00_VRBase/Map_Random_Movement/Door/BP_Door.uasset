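; BP_Door is a damageable door actor with a health bar, in the random movement map folder.
; The construction script picks the Cube's mesh from a Meshes array by ObjectID.
; On BeginPlay it resets Hp to HpMax and registers itself as the Unit of its UI_HPBar widget.
; AnyDamage only subtracts damage from Hp, with no clamping or destruction logic here.
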(event `self.ReceiveBeginPlay`
  (set `self.Hp` (`self.Hp_Max`))
  (bind _asui_hpbar (cast `/Game/00_VRBase/Map_Random_Movement/Door/UI_HPBar` (`WidgetComponent.GetWidget` (`self.Widget`))))
  (set `/Game/00_VRBase/Map_Random_Movement/Door/UI_HPBar.Unit` self _asui_hpbar))

(event `self.ReceiveAnyDamage`
  (params (Damage :type "Float (single-precision)") (DamageType :type "DamageType Object Reference") (InstigatedBy :type "Controller Object Reference") (DamageCauser :type "Actor Object Reference"))
  (set `self.Hp` (- (`self.Hp`) Damage)))

(fn `UserConstructionScript`
  (`StaticMeshComponent.SetStaticMesh` (`self.Cube`) (`|GetArrayItem` (`self.Meshes`) (`self.ObjectID`))))