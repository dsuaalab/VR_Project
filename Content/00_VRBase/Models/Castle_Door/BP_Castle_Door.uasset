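; BP_Castle_Door is a destructible castle door that shows progressive damage as it loses health.
; AnyDamage subtracts incoming damage from HP.
; Tick polls HP against InitHP and shows one of three static meshes for full, half or quarter health by toggling visibility.
; The actor destroys itself on the tick after HP reaches zero.
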(event `self.ReceiveBeginPlay`
  (`SceneComponent.SetVisibility` (`self.StaticMesh_100`) true false)
  (`SceneComponent.SetVisibility` (`self.StaticMesh_50`) false false)
  (`SceneComponent.SetVisibility` (`self.StaticMesh_25`) false false))

(event `self.ReceiveTick`
  (params (DeltaSeconds :type "Float (single-precision)"))
  (if (<= (`self.HP`) 0.0)
    (`self.K2_DestroyActor`)
    (elif (<= (/ (`self.HP`) (`self.Init_HP`)) 0.25)
      (`SceneComponent.SetVisibility` (`self.StaticMesh_100`) false false)
      (`SceneComponent.SetVisibility` (`self.StaticMesh_50`) false false)
      (`SceneComponent.SetVisibility` (`self.StaticMesh_25`) true false)
      (elif (<= (/ (`self.HP`) (`self.Init_HP`)) 0.5)
        (`SceneComponent.SetVisibility` (`self.StaticMesh_100`) false false)
        (`SceneComponent.SetVisibility` (`self.StaticMesh_50`) true false)
        (`SceneComponent.SetVisibility` (`self.StaticMesh_25`) false false)
        (else
          (`SceneComponent.SetVisibility` (`self.StaticMesh_100`) true false)
          (`SceneComponent.SetVisibility` (`self.StaticMesh_50`) false false)
          (`SceneComponent.SetVisibility` (`self.StaticMesh_25`) false false))))))

(event `self.ReceiveAnyDamage`
  (params (Damage :type "Float (single-precision)") (DamageType :type "DamageType Object Reference") (InstigatedBy :type "Controller Object Reference") (DamageCauser :type "Actor Object Reference"))
  (set `self.HP` (- (`self.HP`) Damage)))

(fn `UserConstructionScript`)